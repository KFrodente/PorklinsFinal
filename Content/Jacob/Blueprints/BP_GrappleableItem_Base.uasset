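; Base actor for grappleable items, with empty Pull and SetGrappled events and a GetDoSlowmo function that returns false.
; It caches the player pawn on BeginPlay and line-traces from its Spotlight to the player every tick.
; When the trace hits nothing, the Spotlight rotates along the player-to-light direction, so it faces away from the player.
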(event EventBeginPlay
  (bind _asbp_player (Utilities|Casting|CastToBP_Player (Game|Player|GetPlayerPawn 0)))
  (Variables|Default|SetPlayer _asbp_player))

(event Collision|EventActorBeginOverlap
  (params (OtherActor :type Actor%20Object%20Reference)))

(event EventTick
  (params (DeltaSeconds :type Float%20%28single-precision%29))
  (bind _returnvalue (Collision|LineTraceForObjects (Transformation|GetWorldLocation (Variables|Default|GetSpotlight)) (Transformation|GetActorLocation (Variables|Default|GetPlayer)) (Variables|Default|GetObject%20Types) false 0 "None"))
  (if (not _returnvalue)
    (Transformation|SetWorldRotation (Variables|Default|GetSpotlight) (Math|Rotator|FindLookatRotation (Transformation|GetActorLocation (Variables|Default|GetPlayer)) (Transformation|GetWorldLocation (Variables|Default|GetSpotlight))) false false)))

(event EventPull
  (params (Direction :type Vector :default "0, 0, 0")))

(event EventSetGrappled
  (params (Grappled :type Boolean)))

(fn ConstructionScript)

(fn GetDoSlowmo
  (return false))