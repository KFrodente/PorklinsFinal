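; LevelGate is an actor that moves the player on to the next level when a living BP_Player overlaps it.
; On overlap it sets the player's capsule to ignore Pawn collision and fades in a WBP_LevelTransition widget showing the next level number.
; After a short delay it unpauses and opens the NextLevel reference.
; Disconnected leftover nodes derive the next level from the current level's name.
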(event EventBeginPlay)

(event Collision|EventActorBeginOverlap
  (params (OtherActor :type Actor%20Object%20Reference))
  (bind _asbp_player (Utilities|Casting|CastToBP_Player OtherActor))
  (if (> (Variables|/Game/Jacob/Blueprints/Health.Health_C|GetCurrentHealth (Variables|/Game/Kian/Blueprints/BP_Player.BP_Player_C|GetHealth _asbp_player)) 0)
    (Collision|SetCollisionResponsetoChannel (Variables|/Script/Engine.Character|GetCapsuleComponent _asbp_player) "ECC_Pawn" "ECR_Ignore")
    (bind _returnvalue (UserInterface|CreateWidget "/Game/Jacob/UI/WBP_LevelTransition.WBP_LevelTransition_C"))
    (Rendering|Components|TextRender|SetText (Variables|/Game/Jacob/UI/WBP_LevelTransition.WBP_LevelTransition_C|GetLevelText _returnvalue) (Utilities|Text|FormatText "Level {num}" (+ (Variables|Default|GetThisLevelNumber) 1)))
    (UserInterface|Viewport|AddtoViewport _returnvalue 0)
    (UserInterface|Animation|PlayAnimation _returnvalue (Variables|/Game/Jacob/UI/WBP_LevelTransition.WBP_LevelTransition_C|GetFadeIn _returnvalue) 0.0 1 "Forward" 1.0 false)
    (Utilities|FlowControl|Delay 0.5)
    (Game|SetGamePaused false)
    (Game|OpenLevel(byObjectReference) (Variables|Default|GetNextLevel))))

(event EventTick
  (params (DeltaSeconds :type Float%20%28single-precision%29)))

(fn ConstructionScript)