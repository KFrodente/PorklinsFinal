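; Breakable surface actor that is destroyed by any damage, spawning a hit particle and playing an attenuated metal sound at its location.
; It caches the player pawn on BeginPlay and, while that is valid, flips the particle's yaw based on an X-location comparison.
; GetDoSlowmo always returns true, while the Pull and SetGrappled events are left empty.
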(event EventBeginPlay
  (bind _asbp_player (Utilities|Casting|CastToBP_Player (Game|Player|GetPlayerPawn 0)))
  (Variables|Default|SetPlayer _asbp_player))

(event Collision|EventActorBeginOverlap
  (params (OtherActor :type Actor%20Object%20Reference)))

(event EventTick
  (params (DeltaSeconds :type Float%20%28single-precision%29)))

(event EventPull
  (params (Direction :type Vector :default "0, 0, 0")))

(event EventSetGrappled
  (params (Grappled :type Boolean)))

(event Game|Damage|EventAnyDamage
  (params (Damage :type Float%20%28single-precision%29) (DamageType :type Damage%20Type%20Object%20Reference) (InstigatedBy :type Controller%20Object%20Reference) (DamageCauser :type Actor%20Object%20Reference))
  (Utilities|IsValid (Variables|Default|GetPlayer)
    (:Is%20Valid
      (if (> (.x (Transformation|GetActorLocation)) (.x (Transformation|GetActorLocation)))
        (Variables|Default|SetParticleAngle 0.0)
        (else
          (Variables|Default|SetParticleAngle 1.8e+02)))
      (Niagara|SpawnSystematLocation (Variables|Default|GetHitParticle) (Transformation|GetActorLocation self) (Math|Rotator|MakeRotator 0.0 0.0 (Variables|Default|GetParticleAngle))))
    (:Is%20Not%20Valid
      (Niagara|SpawnSystematLocation (Variables|Default|GetHitParticle) (Transformation|GetActorLocation))))
  (Audio|PlaySoundatLocation "/Game/Jacob/Sounds/Metal2.Metal2" (Transformation|GetActorLocation) "0, 0, 0" 1.0 1.0 0.0 "/Game/Jacob/Sounds/NewSoundAttenuation.NewSoundAttenuation" 0 0 0)
  (Actor|DestroyActor))

(fn ConstructionScript)

(fn GetDoSlowmo
  (return true))