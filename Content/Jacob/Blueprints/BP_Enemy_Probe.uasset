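; BP_Enemy_Probe is a laser-shooting probe enemy that extends a parent enemy Blueprint with bobbing sine movement.
; Its patrol and player-spotted movement overrides call the parent first and add sine motion on success, also turning the sprite toward the player once spotted.
; The attack override fires a laser from a fire point with a shoot sound when the parent allows it.
; An event also stores a grappled flag.
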(event EventBeginPlay
  (|CallParentFunction) ; This node is disabled and will not be called.\nDrag off pins to build functionality.
)

(event Collision|EventActorBeginOverlap
  (params (OtherActor :type Actor%20Object%20Reference))
  (|CallParentFunction OtherActor) ; This node is disabled and will not be called.\nDrag off pins to build functionality.
)

(event EventTick
  (params (DeltaSeconds :type Float%20%28single-precision%29))
  (|CallParentFunction DeltaSeconds) ; This node is disabled and will not be called.\nDrag off pins to build functionality.
)

(event EventSetGrappled
  (params (Grappled :type Boolean))
  (Variables|Default|SetGrappled Grappled))

(fn ConstructionScript
  (|CallParentFunction))

(fn HandlePatrolMovement
  (bind _continue (|CallParentFunction))
  (if _continue
    (CallFunction|DoSinMovement)))

(fn HandlePlayerSpottedMovement
  (bind _player (Variables|Default|Getplayer))
  (bind _continue (|CallParentFunction))
  (if _continue
    (CallFunction|DoSinMovement)
    (Utilities|IsValid _player
      (:Is%20Valid
        (Transformation|SetWorldRotation (Variables|Default|GetSprite) (Math|Rotator|FindLookatRotation (Transformation|GetActorLocation) (Transformation|GetActorLocation _player)) false false)))))

(fn AttackPlayer
  (bind _continue (|CallParentFunction))
  (if _continue
    (CallFunction|ShootLaseratPlayer (Transformation|GetWorldLocation (Variables|Default|GetFirePoint)) self)
    (CallFunction|PlayShootSound)))