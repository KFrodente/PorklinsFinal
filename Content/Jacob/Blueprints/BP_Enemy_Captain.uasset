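; Captain enemy for a side-on sprite game that patrols, then aims and fires lasers at the player.
; Extends parent patrol, spotted and attack functions, with a looping timer reversing the patrol.
; Once the player is spotted, it flips capsule and arm sprite toward them, pitches the arm to aim and holds a middle distance.
; Pull launches it with gravity briefly switched off.
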(event Custom|ChangeDirection
  (bind _capsulecomponent (Variables|Default|GetCapsuleComponent))
  (bind _arm_sprite (Variables|Default|GetArm_Sprite))
  (bind _returnvalue (Transformation|GetWorldRotation _capsulecomponent))
  (bind _relativelocation (Variables|/Script/Engine.SceneComponent|GetRelativeLocation _arm_sprite))
  (if (not (Variables|Default|GetplayerSpotted)) ; Patrolling?
    (if (> (.yaw _returnvalue) 0.0)
      (Transformation|SetWorldRotation _capsulecomponent (Math|Rotator|MakeRotator (.roll _returnvalue) (.pitch _returnvalue) 0.0) false false)
      (Transformation|SetRelativeLocation _arm_sprite (Math|Vector|MakeVector (.x _relativelocation) 1.0 (.z _relativelocation)) false false)
      (else
        (Transformation|SetWorldRotation _capsulecomponent (Math|Rotator|MakeRotator (.roll _returnvalue) (.pitch _returnvalue) 1.8e+02) false false)
        (Transformation|SetRelativeLocation _arm_sprite (Math|Vector|MakeVector (.x _relativelocation) -1.0 (.z _relativelocation)) false false)))))

(event EventBeginPlay
  (|CallParentFunction)
  (Utilities|Time|SetTimerbyEvent (delegate Custom|ChangeDirection) (Variables|Default|GetchangeDirectionTime) true))

(event Collision|EventActorBeginOverlap
  (params (OtherActor :type Actor%20Object%20Reference))
  (|CallParentFunction OtherActor) ; This node is disabled and will not be called.\nDrag off pins to build functionality.
)

(event EventTick
  (params (DeltaSeconds :type Float%20%28single-precision%29))
  (|CallParentFunction DeltaSeconds) ; This node is disabled and will not be called.\nDrag off pins to build functionality.
)

(event EventPull
  (params (Direction :type Vector :default "0, 0, 0"))
  (bind _charactermovement (Variables|Character|GetCharacterMovement))
  (Variables|/Script/Engine.CharacterMovementComponent|SetGravityScale _charactermovement 0.0)
  (Character|LaunchCharacter Direction true true)
  (Utilities|FlowControl|Delay 0.5)
  (Variables|/Script/Engine.CharacterMovementComponent|SetGravityScale _charactermovement 1.0))

(fn ConstructionScript
  (|CallParentFunction))

(fn HandlePatrolMovement
  (bind _continue (|CallParentFunction))
  (if _continue
    (Pawn|Input|AddMovementInput (Transformation|GetActorForwardVector) 1.0 false)
    (Transformation|SetRelativeRotation (Variables|Default|GetArmArrow) (Math|Rotator|MakeRotator 0.0 (Variables|Default|GetrestingArmDegrees) 0.0) false false)))

(fn HandlePlayerSpottedMovement
  (bind _arm_sprite (Variables|Default|GetArm_Sprite))
  (bind _player (Variables|Default|Getplayer))
  (bind _armarrow (Variables|Default|GetArmArrow))
  (bind _capsulecomponent (Variables|Default|GetCapsuleComponent))
  (bind _armarrow_2 (Variables|Default|GetArmArrow))
  (bind _returnvalue (Transformation|GetActorLocation _player))
  (bind _returnvalue_2 (Transformation|GetWorldLocation _armarrow_2))
  (bind _returnvalue_3 (Transformation|GetWorldRotation _capsulecomponent))
  (bind _relativelocation (Variables|/Script/Engine.SceneComponent|GetRelativeLocation _arm_sprite))
  (bind _returnvalue_4 (Math|Rotator|FindLookatRotation _returnvalue_2 _returnvalue))
  (bind _continue (|CallParentFunction))
  (if _continue
    (Utilities|FlowControl|Sequence
      (:then_0
        (bind _onright (CallFunction|PlayeronRight?))
        (if _onright
          (Transformation|SetWorldRotation _armarrow (Math|Rotator|MakeRotator 0.0 (.pitch _returnvalue_4) 0.0) false false)
          (Transformation|SetWorldRotation _capsulecomponent (Math|Rotator|MakeRotator (.roll _returnvalue_3) (.pitch _returnvalue_3) 0.0) false false)
          (Transformation|SetRelativeLocation _arm_sprite (Math|Vector|MakeVector (.x _relativelocation) 1.0 (.z _relativelocation)) false false)
          (else
            (Transformation|SetWorldRotation _armarrow (Math|Rotator|MakeRotator 0.0 (.pitch _returnvalue_4) 1.8e+02) false false)
            (Transformation|SetWorldRotation _capsulecomponent (Math|Rotator|MakeRotator (.roll _returnvalue_3) (.pitch _returnvalue_3) 1.8e+02) false false)
            (Transformation|SetRelativeLocation _arm_sprite (Math|Vector|MakeVector (.x _relativelocation) -1.0 (.z _relativelocation)) false false))))
      (:then_1
        (if (> (Variables|Default|GetplayerDistance) 8e+02)
          (Pawn|Input|AddMovementInput (Transformation|GetActorForwardVector) 1.0 false)
          (elif (< (Variables|Default|GetplayerDistance) 6e+02)
            (Pawn|Input|AddMovementInput (Math|Vector|NegateVector (Transformation|GetActorForwardVector)) 1.0 false)))))))

(fn AttackPlayer
  (bind _continue (|CallParentFunction))
  (if _continue
    (CallFunction|ShootLaseratPlayer (Transformation|GetWorldLocation (Variables|Default|GetActualFirePoint)) self)
    (Audio|PlaySoundatLocation "/Game/Jacob/Sounds/Shoot2.Shoot2" (Transformation|GetActorLocation) "0, 0, 0" 1.0 1.0 0.0 "/Game/Jacob/Sounds/NewSoundAttenuation.NewSoundAttenuation" 0 0 0)
    (return _continue)))