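; BP_Enemy_Drone1 is a flying sprite-based enemy drone that patrols in circles and shoots lasers at the player.
; It overrides parent patrol, spotted and attack functions, extending each only when the parent returns true.
; Once the player is spotted, it flips its sprite toward them.
; While aim pitch stays below a small upward limit, it points GunArrow at the player, holds a height band, and approaches, circles or adjusts horizontally by distance.
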(event EventBeginPlay
  (|CallParentFunction)
  (Pawn|Components|CharacterMovement|SetMovementMode (Variables|Character|GetCharacterMovement) "MOVE_Flying" 0))

(event Collision|EventActorBeginOverlap
  (params (OtherActor :type Actor%20Object%20Reference))
  (|CallParentFunction OtherActor) ; This node is disabled and will not be called.\nDrag off pins to build functionality.
)

(event EventTick
  (params (DeltaSeconds :type Float%20%28single-precision%29))
  (|CallParentFunction DeltaSeconds) ; This node is disabled and will not be called.\nDrag off pins to build functionality.
)

(fn ConstructionScript
  (|CallParentFunction))

(fn HandlePatrolMovement
  (bind _continue (|CallParentFunction))
  (if _continue
    (CallFunction|DoCircleMovement)
    (return _continue)))

(fn HandlePlayerSpottedMovement
  (bind _returnvalue (Transformation|GetActorLocation))
  (bind _returnvalue_2 (Transformation|GetActorLocation))
  (bind _sprite (Variables|Default|GetSprite))
  (bind _player (Variables|Default|Getplayer))
  (bind _gunarrow (Variables|Default|GetGunArrow))
  (bind _player_2 (Variables|Default|Getplayer))
  (bind _player_3 (Variables|Default|Getplayer))
  (bind _returnvalue_3 (Transformation|GetWorldLocation _gunarrow))
  (bind _returnvalue_4 (Transformation|GetActorLocation _player_3))
  (bind _returnvalue_5 (Transformation|GetActorLocation _player_2))
  (bind _returnvalue_6 (Transformation|GetActorLocation _player))
  (bind _returnvalue_7 (Math|Rotator|FindLookatRotation _returnvalue_3 _returnvalue_4))
  (bind _returnvalue_8 (- _returnvalue_5 _returnvalue_2))
  (bind _returnvalue_9 (- (.z _returnvalue) (.z _returnvalue_6)))
  (bind _continue (|CallParentFunction))
  (if _continue
    (Utilities|IsValid (Variables|Default|Getplayer)
      (:Is%20Valid
        (bind _onright (CallFunction|PlayeronRight?))
        (if _onright
          (Transformation|SetWorldRotation _sprite "0, 0, 0" false false)
          (else
            (Transformation|SetWorldRotation _sprite "0.000000,180.000000,0.000000" false false)))
        (if (< (.pitch _returnvalue_7) 5.0)
          (Transformation|SetWorldRotation (Variables|Default|GetGunArrow) (Math|Rotator|MakeRotator (.roll _returnvalue_7) (.pitch _returnvalue_7) (.yaw _returnvalue_7)) false false)
          (Utilities|FlowControl|Sequence
            (:then_0
              (if (> _returnvalue_9 6e+02)
                (Pawn|Input|AddMovementInput "0.000000,0.000000,-0.700000" 1.0 false)
                (elif (< _returnvalue_9 2e+02)
                  (Pawn|Input|AddMovementInput "0.000000,0.000000,0.700000" 1.0 false))))
            (:then_1
              (if (> (Variables|Default|GetplayerDistance) 6e+02)
                (Pawn|Input|AddMovementInput (Math|Vector|MakeVector (.x _returnvalue_8) 0.0 1.0) 1.0 false)
                (elif (> (Variables|Default|GetplayerDistance) 2e+02)
                  (CallFunction|DoSmallCircles)
                  (else
                    (bind _result (Math|Float|NegateFloat (.x _returnvalue_8))
                      (:%20%20
                        (Pawn|Input|AddMovementInput (Math|Vector|MakeVector _result 0.0 0.0) 1.0 false)))))))))))))

(fn AttackPlayer
  (bind _continue (|CallParentFunction))
  (if _continue
    (CallFunction|ShootLaseratPlayer (Transformation|GetWorldLocation (Variables|Default|GetArrow1)) self)
    (return _continue)))