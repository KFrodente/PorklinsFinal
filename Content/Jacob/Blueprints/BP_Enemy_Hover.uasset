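; BP_Enemy_Hover is a hovering enemy that moves back and forth along the X axis and fires lasers at the player.
; It extends its parent's patrol and player-spotted movement with a sine motion and HoverMovement.
; HoverMovement adds horizontal input and reverses direction when a line trace along the travel direction detects an obstacle.
; Its attack spawns BP_Laser from the left or right fire point, depending on the player's side.
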(event EventBeginPlay
  (|CallParentFunction) ; This node is disabled and will not be called.\nDrag off pins to build functionality.
)

(event Collision|EventActorBeginOverlap
  (params (OtherActor :type Actor%20Object%20Reference))
  (|CallParentFunction OtherActor) ; This node is disabled and will not be called.\nDrag off pins to build functionality.
)

(event EventTick
  (params (DeltaSeconds :type Float%20%28single-precision%29))
  (|CallParentFunction DeltaSeconds) ; This node is disabled and will not be called.\nDrag off pins to build functionality.
)

(fn ConstructionScript
  (|CallParentFunction))

(fn HandlePatrolMovement
  (bind _continue (|CallParentFunction))
  (if _continue
    (CallFunction|DoSinMovement)
    (CallFunction|HoverMovement)
    (return _continue)))

(fn HandlePlayerSpottedMovement
  (bind _continue (|CallParentFunction))
  (if _continue
    (CallFunction|DoSinMovement)
    (CallFunction|HoverMovement)
    (return _continue)))

(fn AttackPlayer
  (bind _continue (|CallParentFunction))
  (if _continue
    (bind _onright (CallFunction|PlayeronRight?))
    (if _onright
      (Game|SpawnActorfromClass "/Game/Jacob/Blueprints/BP_Laser.BP_Laser_C" (Transformation|GetWorldTransform (Variables|Default|GetRightFirePoint)) "Undefined" "OverrideRootScale" 0 0)
      (else
        (Game|SpawnActorfromClass "/Game/Jacob/Blueprints/BP_Laser.BP_Laser_C" (Transformation|GetWorldTransform (Variables|Default|GetLeftFirePoint)) "Undefined" "OverrideRootScale" 0 0)))
    (return true)))

(fn HoverMovement
  (bind _returnvalue (Transformation|GetActorLocation))
  (bind _returnvalue_2 (Transformation|GetActorLocation))
  (bind _avoidobjects (Variables|Default|GetAvoidObjects))
  (if (Variables|Default|GetmovingRight)
    (Pawn|Input|AddMovementInput "1.000000,0.000000,0.000000" 1.0 false)
    (bind _returnvalue_3 (Collision|LineTraceForObjects _returnvalue_2 (+ _returnvalue_2 (* (Transformation|GetActorForwardVector) 4e+02)) _avoidobjects false 0 "None" true "(R=1.000000,G=0.000000,B=0.000000,A=1.000000)" "(R=0.000000,G=1.000000,B=0.000000,A=1.000000)" 2.0))
    (if _returnvalue_3
      (Variables|Default|SetmovingRight (not (Variables|Default|GetmovingRight)) :!label _label))
    (else
      (Pawn|Input|AddMovementInput "-1.000000,0.000000,0.000000" 1.0 false)
      (bind _returnvalue_4 (Collision|LineTraceForObjects _returnvalue (+ _returnvalue (* (Math|Vector|NegateVector (Transformation|GetActorForwardVector)) 4e+02)) _avoidobjects false 0 "None" true "(R=1.000000,G=0.000000,B=0.000000,A=1.000000)" "(R=0.000000,G=1.000000,B=0.000000,A=1.000000)" 2.0))
      (if _returnvalue_4
        (goto _label)))))