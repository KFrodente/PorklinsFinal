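; BP_Enemy_Drone is a flying enemy that extends a parent enemy's patrol, spotted and attack behavior.
; Its movement overrides call the parent, then add a sine-driven vertical bob based on game time, with patrol bobbing only when the parent call returns true.
; Once it spots the player, it also rotates its sprite to face them.
; Attacks fire a laser, and a SetGrappled event stores its grappled state.
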(event EventBeginPlay
  (|CallParentFunction) ; This node is disabled and will not be called.\nDrag off pins to build functionality.
)

(event Collision|EventActorBeginOverlap
  (params (OtherActor :type Actor%20Object%20Reference))
  (|CallParentFunction OtherActor) ; This node is disabled and will not be called.\nDrag off pins to build functionality.
)

(event EventTick
  (params (DeltaSeconds :type Float%20%28single-precision%29))
  (|CallParentFunction DeltaSeconds) ; This node is disabled and will not be called.\nDrag off pins to build functionality.
)

(event EventSetGrappled
  (params (Grappled :type Boolean))
  (Variables|Default|SetGrappled Grappled))

(fn ConstructionScript
  (|CallParentFunction))

(fn HandlePatrolMovement
  (bind _returnvalue (Transformation|GetActorLocation))
  (bind _continue (|CallParentFunction))
  (if _continue
    (Transformation|SetActorLocation (Math|Vector|MakeVector (.x _returnvalue) (.y _returnvalue) (+ (.z _returnvalue) (* (Math|Trig|Sin(Degrees) (* (Utilities|Time|GetGameTimeinSeconds) 75.0)) 2.0))) false false)))

(fn HandlePlayerSpottedMovement
  (bind _returnvalue (Transformation|GetActorLocation))
  (bind _player (Variables|Default|Getplayer))
  (|CallParentFunction)
  (Transformation|SetActorLocation (Math|Vector|MakeVector (.x _returnvalue) (.y _returnvalue) (+ (.z _returnvalue) (* (Math|Trig|Sin(Degrees) (* (Utilities|Time|GetGameTimeinSeconds) 75.0)) 2.0))) false false)
  (Utilities|IsValid _player
    (:Is%20Valid
      (Transformation|SetWorldRotation (Variables|Default|GetSprite) (Math|Rotator|FindLookatRotation (Transformation|GetActorLocation) (Transformation|GetActorLocation _player)) false false))))

(fn AttackPlayer
  (|CallParentFunction)
  (CallFunction|ShootLaseratPlayer))