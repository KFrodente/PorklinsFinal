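; Stationary turret enemy that aims at the player and fires lasers, built on a parent enemy class.
; Tick zeroes character movement velocity to hold it in place.
; When the parent's spotted-movement check passes, the barrel arrow pitches toward the player with yaw snapped left or right, side-scroller style.
; When the parent's attack check passes, it shoots a laser from the fire point and prints a debug string.
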(event EventBeginPlay
  (|CallParentFunction) ; This node is disabled and will not be called.\nDrag off pins to build functionality.
)

(event Collision|EventActorBeginOverlap
  (params (OtherActor :type Actor%20Object%20Reference))
  (|CallParentFunction OtherActor) ; This node is disabled and will not be called.\nDrag off pins to build functionality.
)

(event EventTick
  (params (DeltaSeconds :type Float%20%28single-precision%29))
  (|CallParentFunction DeltaSeconds)
  (Variables|/Script/Engine.MovementComponent|SetVelocity (Variables|Character|GetCharacterMovement) "0, 0, 0"))

(fn ConstructionScript
  (|CallParentFunction))

(fn AttackPlayer
  (bind _continue (|CallParentFunction))
  (if _continue
    (CallFunction|ShootLaseratPlayer (Transformation|GetWorldLocation (Variables|Default|GetActualFirePoint)) self)
    (Development|PrintString "Hello")
    (return _continue)))

(fn HandlePlayerSpottedMovement
  (bind _barrelarrow (Variables|Default|GetBarrelArrow))
  (bind _player (Variables|Default|Getplayer))
  (bind _barrelarrow_2 (Variables|Default|GetBarrelArrow))
  (bind _returnvalue (Transformation|GetWorldLocation _barrelarrow))
  (bind _returnvalue_2 (Transformation|GetActorLocation _player))
  (bind _returnvalue_3 (Math|Rotator|FindLookatRotation _returnvalue _returnvalue_2))
  (bind _continue (|CallParentFunction))
  (if _continue
    (bind _onright (CallFunction|PlayeronRight?))
    (if _onright
      (Transformation|SetWorldRotation _barrelarrow_2 (Math|Rotator|MakeRotator 0.0 (.pitch _returnvalue_3) 0.0) false false)
      (else
        (Transformation|SetWorldRotation _barrelarrow_2 (Math|Rotator|MakeRotator 0.0 (.pitch _returnvalue_3) 1.8e+02) false false)))
    (return _continue)))