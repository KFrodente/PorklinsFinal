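; Base enemy for a side-view game that patrols, spots the player and attacks, with stub movement and attack functions that only report whether it is ungrappled.
; A looping timer fans out line traces as cone vision; Tick then runs cooldown-gated attacks until the player leaves three times vision range.
; It handles grapple pulls with decaying velocity, and damage with directional particles and death.
; Shared helpers provide laser shots and sine or circular motion.
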(event Custom|Patrol
  (if (not (Variables|Default|GetplayerSpotted))
    (|ConeVisionSearch)))

(event Custom|Slowdown
  (bind _charactermovement (Variables|Character|GetCharacterMovement))
  (bind _output_get (Variables|/Script/Engine.MovementComponent|SetVelocity _charactermovement (* (Variables|/Script/Engine.MovementComponent|GetVelocity _charactermovement) 0.8)))
  (if (Utilities|Operators|EqualEqual :A _output_get :ErrorTolerance 5e+01)
    (Variables|/Script/Engine.MovementComponent|SetVelocity _charactermovement "0, 0, 0")
    (Utilities|Time|ClearandInvalidateTimerbyHandle (Variables|Default|GetSlowdownTimer))))

(event EventBeginPlay
  (Utilities|Time|SetTimerbyEvent (delegate Custom|Patrol) 0.3 true))

(event Collision|EventActorBeginOverlap
  (params (OtherActor :type Actor%20Object%20Reference)))

(event EventTick
  (params (DeltaSeconds :type Float%20%28single-precision%29))
  (if (Variables|Default|GetplayerSpotted)
    (|WhenSpottedPlayer)
    (else
      (CallFunction|HandlePatrolMovement))))

(event EventPull
  (params (Direction :type Vector :default "0, 0, 0"))
  (Character|LaunchCharacter Direction true true)
  (Utilities|FlowControl|Delay 0.1)
  (bind _returnvalue (Utilities|Time|SetTimerbyEvent (delegate Custom|Slowdown) 0.1 true))
  (Variables|Default|SetSlowdownTimer _returnvalue))

(event Game|Damage|EventAnyDamage
  (params (Damage :type Float%20%28single-precision%29) (DamageType :type Damage%20Type%20Object%20Reference) (InstigatedBy :type Controller%20Object%20Reference) (DamageCauser :type Actor%20Object%20Reference))
  (bind _health (Variables|Default|GetHealth))
  (bind _onright (CallFunction|PlayeronRight?))
  (if _onright
    (Variables|Default|SetParticleAngle 0.0)
    (else
      (Variables|Default|SetParticleAngle 1.8e+02)))
  (Niagara|SpawnSystematLocation (Variables|Default|GetHitParticle) (Transformation|GetActorLocation self) (Math|Rotator|MakeRotator 0.0 0.0 (Variables|Default|GetParticleAngle)))
  (bind _output_get (Variables|/Game/Jacob/Blueprints/Health.Health_C|SetCurrentHealth _health (Math|Float|Truncate (- (Variables|/Game/Jacob/Blueprints/Health.Health_C|GetCurrentHealth _health) Damage))))
  (if (<= _output_get 0)
    (Actor|DestroyActor)))

(event EventSetGrappled
  (params (Grappled :type Boolean))
  (Variables|Default|SetGrappled Grappled))

(fn ConstructionScript)

(fn AttackPlayer
  (return (not (Variables|Default|GetGrappled))))

(fn HandlePlayerSpottedMovement
  (Variables|Default|SetplayerDistance (Math|Vector|Distance2D(Vector) (Math|Conversions|ToVector2D(Vector) (Transformation|GetActorLocation)) (Math|Conversions|ToVector2D(Vector) (Transformation|GetActorLocation (Variables|Default|Getplayer)))))
  (return (not (Variables|Default|GetGrappled))))

(fn HandlePatrolMovement
  (return (not (Variables|Default|GetGrappled))))

(fn ShootLaseratPlayer
  (params (SpawnLocation :type Vector) (PersonWhoShot :type Actor%20Object%20Reference))
  (bind _returnvalue (Transformation|GetActorLocation))
  (bind _player (Variables|Default|Getplayer))
  (bind _returnvalue_2 (Transformation|GetActorLocation _player))
  (Utilities|IsValid (Variables|Default|Getplayer)
    (:Is%20Valid
      (if (Utilities|Operators|EqualEqual :A SpawnLocation)
        (Game|SpawnActorfromClass "/Game/Jacob/Blueprints/BP_Laser.BP_Laser_C" (Math|Transform|MakeTransform _returnvalue (Math|Rotator|FindLookatRotation _returnvalue _returnvalue_2) "1.000000,1.000000,1.000000") "Undefined" "MultiplyWithRoot" PersonWhoShot 0)
        (else
          (Game|SpawnActorfromClass "/Game/Jacob/Blueprints/BP_Laser.BP_Laser_C" (Math|Transform|MakeTransform SpawnLocation (Math|Rotator|FindLookatRotation SpawnLocation _returnvalue_2) "1.000000,1.000000,1.000000") "Undefined" "MultiplyWithRoot" PersonWhoShot 0))))))

(fn DoSinMovement
  (bind _returnvalue (Transformation|GetActorLocation))
  (Transformation|SetActorLocation (Math|Vector|MakeVector (.x _returnvalue) (.y _returnvalue) (+ (.z _returnvalue) (* (Math|Trig|Sin(Degrees) (* (Utilities|Time|GetGameTimeinSeconds) (Variables|Default|GetSinSpeed))) (Variables|Default|GetSinAmplitude)))) false false))

(fn PlayeronRight?
  (bind _player (Variables|Default|Getplayer))
  (Utilities|IsValid _player
    (:Is%20Valid
      (if (> (.x (Transformation|GetActorLocation _player)) (.x (Transformation|GetActorLocation))) ; Player on right?
        (return true)
        (else
          (return false))))))

(fn DoCircleMovement
  (bind _returnvalue (Transformation|GetActorLocation))
  (Transformation|SetActorLocation (Math|Vector|MakeVector (+ (.x (Transformation|GetActorLocation)) (* (Math|Trig|Cos(Degrees) (* (Utilities|Time|GetGameTimeinSeconds) (Variables|Default|GetCosSpeed))) (Variables|Default|GetCosAmplitude))) (.y _returnvalue) (+ (.z _returnvalue) (* (Math|Trig|Sin(Degrees) (* (Utilities|Time|GetGameTimeinSeconds) (Variables|Default|GetSinSpeed))) (Variables|Default|GetSinAmplitude)))) false false))

(fn DoSmallCircles
  (bind _returnvalue (Transformation|GetActorLocation))
  (Transformation|SetActorLocation (Math|Vector|MakeVector (+ (.x (Transformation|GetActorLocation)) (* (Math|Trig|Cos(Degrees) (* (Utilities|Time|GetGameTimeinSeconds) 1e+02)) 1.0)) (.y _returnvalue) (+ (.z _returnvalue) (* (Math|Trig|Sin(Degrees) (* (Utilities|Time|GetGameTimeinSeconds) 1e+02)) 1.0))) false false))

(fn GetDoSlowmo
  (return true))