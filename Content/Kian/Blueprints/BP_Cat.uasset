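; BP_Cat is a cat actor that meows at the player and can show rainbow lights.
; When a BP_Player begins overlapping it, it plays a random sound from the Meows array as non-positional 2D audio.
; While RainbowLights is enabled, Tick colors the left and right spotlights from a Hue value that increases each frame without an explicit wrap, so the cycle speed depends on frame rate.
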(event Collision|EventActorBeginOverlap
  (params (OtherActor :type Actor%20Object%20Reference))
  (Utilities|Casting|CastToBP_Player OtherActor)
  (Audio|PlaySound2D (.OutItem (Utilities|Array|Random (Variables|Default|GetMeows))) 2.0 1.0 0.0 0 0))

(event EventTick
  (params (DeltaSeconds :type Float%20%28single-precision%29))
  (if (Variables|Default|GetRainbowLights)
    (Rendering|Components|Light|SetLightColor (Variables|Default|GetSpotLightLeft) (Class|KismetMathLibrary|HSVtoRGB (Variables|Default|GetHue) 1.0 1.0 1.0) false)
    (Rendering|Components|Light|SetLightColor (Variables|Default|GetSpotLightRight) (Class|KismetMathLibrary|HSVtoRGB (Variables|Default|GetHue) 1.0 1.0 1.0) false)
    (Variables|Default|SetHue (+ (Variables|Default|GetHue) 1.0))))

(fn ConstructionScript)