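; BP_Player is a mouse-aimed side-scrolling character with layered sprites, variable jump gravity, a dashing slash and a grapple.
; Slash damages enemies near the cursor direction, launches the player and refreshes on hit.
; Grapple press finds targets via narrow then wide sphere traces; release launches the player and pulls the target via I_Grappleable.
; Some targets trigger distance-based slow motion and reframe BP_WorldCamera until the next slash.
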(event Custom|ResetSwordSlash
  (bind _returnvalue (Transformation|GetActorLocation))
  (bind _returnvalue_2 (Game|GetPlayerController 0))
  (bind _charactermovement (Variables|Character|GetCharacterMovement))
  (bind (_worldlocation _worlddirection) (Game|Player|ConvertMouseLocationToWorldSpace _returnvalue_2))
  (Utilities|FlowControl|DoOnce false) ; enters at Reset
)

(event Custom|IFrames
  (Collision|SetCollisionResponsetoChannel (Variables|Collision|GetCapsuleComponent) "ECC_Pawn" "ECR_Block"))

(event Input|EnhancedActionEvents|EnhancedInputActionIA_Jump
  (params (ActionValue :type Boolean) (ElapsedSeconds :type Float%20%28double-precision%29) (TriggeredSeconds :type Float%20%28double-precision%29) (InputAction :type Input%20Action%20Object%20Reference :default "/Game/Input/IA_Jump.IA_Jump"))
  (:Started
    (Character|Jump)
    (Variables|/Script/Engine.CharacterMovementComponent|SetGravityScale (Variables|Character|GetCharacterMovement) (Variables|Default|GetOriginalGravity)))
  (:Canceled
    (Character|StopJumping :!label _label)
    (Variables|/Script/Engine.CharacterMovementComponent|SetGravityScale (Variables|Character|GetCharacterMovement) (Variables|Default|GetFallGravity)))
  (:Completed
    (goto _label)))

(event Input|EnhancedActionEvents|EnhancedInputActionIA_Slash
  (params (ActionValue :type Boolean) (ElapsedSeconds :type Float%20%28double-precision%29) (TriggeredSeconds :type Float%20%28double-precision%29) (InputAction :type Input%20Action%20Object%20Reference :default "/Game/Input/IA_Slash.IA_Slash"))
  (bind _returnvalue (Transformation|GetActorLocation))
  (bind _returnvalue_2 (Game|GetPlayerController 0))
  (bind _charactermovement (Variables|Character|GetCharacterMovement))
  (bind (_worldlocation _worlddirection) (Game|Player|ConvertMouseLocationToWorldSpace _returnvalue_2))
  (:Started
    (Utilities|FlowControl|DoOnce false :!label _label
      (:Completed
        (Variables|/Script/PorklinsFinal.WorldCamera|SetFollowPlayer (Variables|Default|GetWorldCamera) true)
        (Utilities|Time|ClearandInvalidateTimerbyHandle (Variables|Default|GetSlowmoTimer))
        (Utilities|FlowControl|Sequence
          (:then_0
            (Variables|/Script/Engine.CharacterMovementComponent|SetGroundFriction (Variables|Character|GetCharacterMovement) 0.0))
          (:then_1
            (Utilities|Time|SetGlobalTimeDilation 1.0)
            (bind _outhit (Collision|LineTraceForObjects _worldlocation (+ _worldlocation (* _worlddirection 5e+03)) (Variables|Default|GetRayWallCheck) false 0 "None" true "(R=1.000000,G=0.000000,B=0.000000,A=1.000000)" "(R=0.000000,G=1.000000,B=0.000000,A=1.000000)" 1.0))
            (bind _outactors (Collision|SphereOverlapActors (+ _returnvalue (* (Math|Vector|Normalize (- (.ImpactPoint (Collision|BreakHitResult _outhit)) _returnvalue)) 1.5e+02)) 1.5e+02 (Variables|Default|GetEnemyCheck) 0))
            (Rendering|Debug|DrawDebugSphere (+ _returnvalue (* (Math|Vector|Normalize (- (.ImpactPoint (Collision|BreakHitResult _outhit)) _returnvalue)) 1.5e+02)) 1.5e+02 12 "(R=1.000000,G=0.000000,B=0.388755,A=1.000000)" 3.0 5.0)
            (for _array_element _outactors
              (Utilities|Casting|CastToI_Slashable _array_element)
              (Game|Damage|ApplyDamage _array_element 1e+01 0 self)
              (Utilities|Time|ClearandInvalidateTimerbyHandle (Variables|Default|GetSlashTimer))
              (goto _label Reset))
            (Character|LaunchCharacter (* (* (Math|Vector|Normalize (- (.ImpactPoint (Collision|BreakHitResult _outhit)) _returnvalue)) 1.5e+02) 15.0) false false)
            (Variables|/Script/Engine.CharacterMovementComponent|SetGravityScale _charactermovement (Variables|Default|GetOriginalGravity))
            (Utilities|FlowControl|Delay 0.2)
            (Variables|/Script/Engine.CharacterMovementComponent|SetGroundFriction _charactermovement 8.0))
          (:then_2
            (bind _returnvalue_3 (Utilities|Time|SetTimerbyEvent (delegate Custom|ResetSwordSlash) 0.5))
            (Variables|Default|SetSlashTimer _returnvalue_3)))))))

(event EventBeginPlay
  (bind _returnvalue (Game|GetPlayerController 0))
  ;[1 1 1] Give player controls
  (bind _asbp_player_controller (Utilities|Casting|CastToBP_PlayerController _returnvalue))
  (Input|AddMappingContext (PlayerController|LocalPlayerSubsystems|GetEnhancedInputLocalPlayerSubsystem _asbp_player_controller) "/Game/Input/IMC_Player.IMC_Player" 0 "(bIgnoreAllPressedKeysUntilRelease=True,bForceImmediately=False,bNotifyUserSettings=False)")
  (Variables|Default|SetOriginalGravity (Variables|/Script/Engine.CharacterMovementComponent|GetGravityScale (Variables|Character|GetCharacterMovement)))
  (Variables|/Script/Engine.PlayerController|SetbShowMouseCursor _returnvalue true)
  (bind _returnvalue_2 (Actor|GetActorOfClass "/Game/Kian/Blueprints/BP_WorldCamera.BP_WorldCamera_C"))
  (Variables|Default|SetWorldCamera _returnvalue_2)
  (Game|Player|SetViewTargetwithBlend (Game|GetPlayerController 0) _returnvalue_2 0.0 "VTBlend_Linear" 0.0 false))

(event Game|Damage|EventAnyDamage
  (params (Damage :type Float%20%28single-precision%29) (DamageType :type Damage%20Type%20Object%20Reference) (InstigatedBy :type Controller%20Object%20Reference) (DamageCauser :type Actor%20Object%20Reference))
  (bind _health (Variables|Default|GetHealth))
  (bind _output_get (Variables|/Game/Jacob/Blueprints/Health.Health_C|SetCurrentHealth _health (Math|Float|Truncate (- (Variables|/Game/Jacob/Blueprints/Health.Health_C|GetCurrentHealth _health) Damage))))
  (Development|PrintString (Utilities|String|ToString(Integer) _output_get))
  (Collision|SetCollisionResponsetoChannel (Variables|Collision|GetCapsuleComponent) "ECC_Pawn" "ECR_Ignore")
  (Utilities|Time|SetTimerbyEvent (delegate Custom|IFrames) 1.0))

(event EventOnLanded
  (params (Hit :type Hit%20Result%20Structure%20%28by%20ref%29))
  (Variables|/Script/Engine.CharacterMovementComponent|SetGravityScale (Variables|Character|GetCharacterMovement) (Variables|Default|GetOriginalGravity)))

(event EventTick
  (params (DeltaSeconds :type Float%20%28single-precision%29))
  (bind _returnvalue (Game|GetPlayerController 0))
  (bind _headsprite (Variables|Default|GetHeadSprite))
  (bind (_worldlocation _worlddirection) (Game|Player|ConvertMouseLocationToWorldSpace _returnvalue))
  (bind _returnvalue_2 (Class|PaperFlipbookComponent|GetFlipbook _headsprite))
  (bind _outhit (Collision|LineTraceForObjects _worldlocation (+ _worldlocation (* _worlddirection 5e+03)) (Variables|Default|GetRayWallCheck) false 0 "None" true "(R=1.000000,G=0.000000,B=0.000000,A=1.000000)" "(R=0.000000,G=1.000000,B=0.000000,A=1.000000)" 1.0))
  (bind _output_get (Variables|Default|SetMousePosition (.impactpoint _outhit)))
  (if (not (and (== _returnvalue_2 "/Game/Bennie/FlipBooks/Player/Run/PF_SamRunHead.PF_SamRunHead") (!= _returnvalue_2 "/Game/Bennie/FlipBooks/Player/Jump/PF_SamJumpBody.PF_SamJumpBody")))
    (Transformation|SetRelativeRotation _headsprite (Math|Rotator|MakeRotator 0.0 (.Pitch (Math|Rotator|BreakRotator (Math|Rotator|FindLookatRotation (Transformation|GetWorldLocation _headsprite) _output_get))) 0.0) false false)
    (if (> (.X (Math|Vector|BreakVector _output_get)) (.x (Transformation|GetActorLocation)))
      (Transformation|SetRelativeRotation (Variables|Default|GetSprite) (Math|Rotator|MakeRotator 0.0 0.0 0.0) false false)
      (else
        (Transformation|SetRelativeRotation (Variables|Default|GetSprite) (Math|Rotator|MakeRotator 0.0 0.0 1.8e+02) false false)))))

(fn ConstructionScript)

(event Input|EnhancedActionEvents|EnhancedInputActionIA_Walk
  (params (ActionValue :type Float%20%28double-precision%29) (ElapsedSeconds :type Float%20%28double-precision%29) (TriggeredSeconds :type Float%20%28double-precision%29) (InputAction :type Input%20Action%20Object%20Reference :default "/Game/Input/IA_Walk.IA_Walk"))
  (bind _armsprite (Variables|Default|GetArmSprite))
  (bind _sprite (Variables|Default|GetSprite))
  (bind _headsprite (Variables|Default|GetHeadSprite))
  (bind _relativelocation (Variables|/Script/Engine.SceneComponent|GetRelativeLocation _armsprite))
  (bind _relativelocation_2 (Variables|/Script/Engine.SceneComponent|GetRelativeLocation _headsprite))
  (:Triggered
    (Pawn|Input|AddMovementInput "1.000000,0.000000,0.000000" ActionValue false)
    (if (> ActionValue 0.0) :!label _label
      (Transformation|SetWorldRotation _sprite "0, 0, 0" false false)
      (Transformation|SetRelativeLocation _armsprite (Math|Vector|MakeVector (.x _relativelocation) 8.0 (.z _relativelocation)) false false)
      (Transformation|SetRelativeLocation _headsprite (Math|Vector|MakeVector (.x _relativelocation_2) 4.0 (.z _relativelocation_2)) false false)
      (else
        (Transformation|SetWorldRotation _sprite "0.000000,180.000000,0.000000" false false)
        (Transformation|SetRelativeLocation _armsprite (Math|Vector|MakeVector (.x _relativelocation) -8.0 (.z _relativelocation)) false false)
        (Transformation|SetRelativeLocation _headsprite (Math|Vector|MakeVector (.x _relativelocation_2) -4.0 (.z _relativelocation_2)) false false))))
  (:Canceled
    (goto _label)))

(event EventOnJumped
  (Class|PaperZDAnimInstance|JumptoNode (Variables|/Script/PaperZD.PaperZDAnimationComponent|GetAnimInstance (Variables|Default|GetAnimationBody)) "Airborne" "Locomotion"))

(event EventOnWalkingOffLedge
  (params (PreviousFloorImpactNormal :type Vector%20%28by%20ref%29 :default "0, 0, 0") (PreviousFloorContactNormal :type Vector%20%28by%20ref%29 :default "0, 0, 0") (PreviousLocation :type Vector%20%28by%20ref%29 :default "0, 0, 0") (TimeDelta :type Float%20%28single-precision%29))
  (Class|PaperZDAnimInstance|JumptoNode (Variables|/Script/PaperZD.PaperZDAnimationComponent|GetAnimInstance (Variables|Default|GetAnimationBody)) "Airborne" "Locomotion"))

(event Custom|ResetGrapple
  (bind _returnvalue (Transformation|GetActorLocation))
  (bind _returnvalue_2 (Transformation|GetActorLocation))
  (bind _returnvalue_3 (Transformation|GetActorLocation))
  (bind _returnvalue_4 (Transformation|GetActorUpVector))
  (bind _returnvalue_5 (Transformation|GetActorLocation))
  (bind _grapple (Variables|Default|GetGrapple))
  (bind _charactermovement (Variables|Character|GetCharacterMovement))
  (bind _worldcamera (Variables|Default|GetWorldCamera))
  (bind _returnvalue_6 (* _returnvalue_4 65.0))
  (bind _returnvalue_7 (+ _returnvalue_6 _returnvalue_2))
  (Utilities|FlowControl|DoOnce false) ; enters at Reset
)

(event Custom|Slowmo
  (Utilities|Time|SetGlobalTimeDilation (Math|Float|Lerp 1.0 0.05 (- 1.0 (Math|Float|Power (/ (Math|Vector|Distance(Vector) (Transformation|GetActorLocation (Variables|Default|GetGrappledActor)) (Transformation|GetActorLocation)) (Variables|Default|GetMaxGrappleDistance)) 2.0)))))

(event Input|EnhancedActionEvents|EnhancedInputActionIA_Grapple
  (params (ActionValue :type Boolean) (ElapsedSeconds :type Float%20%28double-precision%29) (TriggeredSeconds :type Float%20%28double-precision%29) (InputAction :type Input%20Action%20Object%20Reference :default "/Game/Input/IA_Grapple.IA_Grapple"))
  (bind _returnvalue (Transformation|GetActorLocation))
  (bind _returnvalue_2 (Transformation|GetActorLocation))
  (bind _returnvalue_3 (Transformation|GetActorLocation))
  (bind _returnvalue_4 (Transformation|GetActorUpVector))
  (bind _returnvalue_5 (Transformation|GetActorLocation))
  (bind _grapple (Variables|Default|GetGrapple))
  (bind _charactermovement (Variables|Character|GetCharacterMovement))
  (bind _worldcamera (Variables|Default|GetWorldCamera))
  (bind _returnvalue_6 (* _returnvalue_4 65.0))
  (bind _returnvalue_7 (+ _returnvalue_6 _returnvalue_2))
  (:Started
    (Utilities|FlowControl|DoOnce false
      (:Completed
        (Variables|Default|SetGrappledActor 0)
        (Utilities|FlowControl|Sequence
          (:then_0
            (bind (_outhit _returnvalue_8) (Collision|SphereTraceForObjects (+ (* (Transformation|GetActorUpVector) 65.0) _returnvalue) (+ _returnvalue (* (Math|Vector|Normalize (- (Variables|Default|GetMousePosition) (Transformation|GetActorLocation))) (Variables|Default|GetMaxGrappleDistance))) 25.0 (Variables|Default|GetObject%20Types) false 0 "ForDuration" true "(R=1.000000,G=0.000000,B=0.000000,A=1.000000)" "(R=0.000000,G=1.000000,B=0.000000,A=1.000000)" 0.5))
            (if _returnvalue_8
              (bind _asi_grappleable (Utilities|Casting|CastToI_Grappleable (.HitActor (Collision|BreakHitResult _outhit)))
                (:then
                  (Variables|Default|SetGrappleConnectionLocation (.ImpactPoint (Collision|BreakHitResult _outhit)))
                  (Variables|Default|SetGrappledActor (.HitActor (Collision|BreakHitResult _outhit)))
                  (Default|SetGrappled _asi_grappleable true)
                  (goto _label_2 Reset))
                (:CastFailed
                  _)))
            (bind (_outhits _returnvalue_9) (Collision|MultiSphereTraceForObjects _returnvalue_7 (+ _returnvalue_2 (* (Math|Vector|Normalize (- (Variables|Default|GetMousePosition) (Transformation|GetActorLocation))) (Variables|Default|GetMaxGrappleDistance))) 75.0 (Variables|Default|GetObject%20Types) false 0 "ForDuration" true "(R=0.269644,G=0.960190,B=1.000000,A=1.000000)" "(R=0.857712,G=1.000000,B=0.229167,A=1.000000)" 0.5))
            (if _returnvalue_9
              (for _array_element _outhits
                (bind _returnvalue_10 (Collision|LineTraceForObjects _returnvalue_7 (Transformation|GetActorLocation (.HitActor (Collision|BreakHitResult _array_element))) (Variables|Default|GetStaticCheck) false 0 "ForDuration" true "(R=0.723604,G=0.000000,B=1.000000,A=1.000000)" "(R=0.000000,G=1.000000,B=0.000000,A=1.000000)" 1.0))
                (if (not _returnvalue_10)
                  (Utilities|IsValid (Variables|Default|GetGrappledActor)
                    (:Is%20Valid
                      (if (< (Math|Vector|Distance(Vector) (Transformation|GetActorLocation (.HitActor (Collision|BreakHitResult _array_element))) _returnvalue_3) (Math|Vector|Distance(Vector) (Transformation|GetActorLocation (Variables|Default|GetGrappledActor)) _returnvalue_3))
                        (bind _asi_grappleable_2 (Utilities|Casting|CastToI_Grappleable (.HitActor (Collision|BreakHitResult _array_element)) :!label _label))
                        (Variables|Default|SetGrappledActor (.HitActor (Collision|BreakHitResult _array_element)))
                        (Variables|Default|SetGrappleConnectionLocation (Transformation|GetActorLocation (.HitActor (Collision|BreakHitResult _array_element))))
                        (Default|SetGrappled _asi_grappleable_2 true)
                        (goto _label_2 Reset)))
                    (:Is%20Not%20Valid
                      (goto _label)))))
              (else
                (Variables|Default|SetGrappleConnectionLocation (Transformation|GetActorLocation))
                (Variables|Default|SetGrappledActor 0))))
          (:then_1
            (Utilities|Time|SetTimerbyEvent (delegate Custom|ResetGrapple) 0.5))))))
  (:Completed
    (Utilities|FlowControl|DoOnce false :!label _label_2
      (:Completed
        (if (Utilities|IsValid (Variables|Default|GetGrappledActor))
          (Variables|Default|SetGrapplePullStrength (* (+ 0.0 (/ (Math|Vector|Distance(Vector) (Variables|Default|GetGrappleConnectionLocation) (Transformation|GetActorLocation)) (Variables|Default|GetMaxGrappleDistance))) (Variables|Default|GetOGrapplePullStrength)))
          (Utilities|Casting|CastToBP_GrappleableItem_Base (Variables|Default|GetGrappledActor)
            (:then
              (bind _returnvalue_11 (Class|GrappleComponent|GetLaunchDirection _grapple (Variables|Default|GetGrappleConnectionLocation) _returnvalue_5 (* (Variables|Default|GetGrapplePullStrength) 3.0)))
              (Character|LaunchCharacter _returnvalue_11 true true))
            (:CastFailed
              (bind _returnvalue_12 (Class|GrappleComponent|GetLaunchDirection _grapple (Variables|Default|GetGrappleConnectionLocation) _returnvalue_5 (Variables|Default|GetGrapplePullStrength)))
              (Character|LaunchCharacter _returnvalue_12 true true)))
          (bind _returnvalue_13 (Class|GrappleComponent|GetLaunchDirection _grapple _returnvalue_5 (Variables|Default|GetGrappleConnectionLocation) (Variables|Default|GetGrapplePullStrength)))
          (bind _asi_grappleable_3 (Utilities|Casting|CastToI_Grappleable (Variables|Default|GetGrappledActor)))
          (Default|Pull _asi_grappleable_3 _returnvalue_13)
          (Default|SetGrappled _asi_grappleable_3 false)
          (bind _doslowmo (Default|GetDoSlowmo _asi_grappleable_3))
          (if _doslowmo
            (bind _returnvalue_14 (Utilities|Time|SetTimerbyEvent (delegate Custom|Slowmo) 0.01 true))
            (Variables|Default|SetSlowmoTimer _returnvalue_14)
            (Variables|/Script/Engine.CharacterMovementComponent|SetGravityScale _charactermovement 0.0)
            (Variables|/Script/Engine.CharacterMovementComponent|SetGroundFriction _charactermovement 0.0)
            (Class|WorldCamera|GiveWantedValues _worldcamera (Transformation|GetActorLocation) (Transformation|GetActorLocation (Variables|Default|GetGrappledActor)) 1.5e+03)
            (Variables|/Script/PorklinsFinal.WorldCamera|SetFollowPlayer _worldcamera false)))))))